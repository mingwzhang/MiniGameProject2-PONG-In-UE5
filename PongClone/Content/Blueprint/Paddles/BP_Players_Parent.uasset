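; Parent Blueprint for player paddles that handles scoring, match end, pausing and muting.
; AddLeftScore and AddRightScore count points; reaching ScoreToWin destroys the ball spawner and shows that player's win widget.
; After a short delay, BP_NPCExistCheck decides whether the one-player or two-player level is reopened.
; PauseButton toggles a cached pause menu with game pause, cursor and input mode, while M flip-flops between mute and unmute sound mixes.
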(event `AddLeftScore`
  (bind _leftscore (`self.LeftScore`))
  ;[1 1 1] Score, Win Conditions, and Reset Game
  (set `self.LeftScore` (+ _leftscore 1))
  (if (== _leftscore (`self.ScoreToWin`))
    (bind _returnvalue (`GameplayStatics.GetActorOfClass` "/Game/Blueprint/BallsAndGoals/BP_BallSpawner.BP_BallSpawner_C"))
    (`self.K2_DestroyActor` _returnvalue)
    (bind _returnvalue_2 (`|CreateWidget` "/Game/UI/W_Player1Wins.W_Player1Wins_C"))
    (`UserWidget.AddToViewport` _returnvalue_2 0)
    (`KismetSystemLibrary.Delay` 3.0)
    (bind _returnvalue_3 (`GameplayStatics.GetActorOfClass` "/Game/Blueprint/Paddles/BP_NPCExistCheck.BP_NPCExistCheck_C" :!label _label))
    (if (`/Game/Blueprint/Paddles/BP_NPCExistCheck.NPC_Exist` _returnvalue_3)
      (`GameplayStatics.OpenLevel` "L_OnePlayerGame")
      (else
        (`GameplayStatics.OpenLevel` "L_TwoPlayerGame")))))

(event `self.ReceiveBeginPlay`
  (`WidgetBlueprintLibrary.SetFocusToGameViewport`))

(event `AddRightScore`
  (bind _rightscore (`self.RightScore`))
  ;[1 1 1] Score, Win Conditions, and Reset Game
  (set `self.RightScore` (+ _rightscore 1))
  (if (== _rightscore (`self.ScoreToWin`))
    (bind _returnvalue (`GameplayStatics.GetActorOfClass` "/Game/Blueprint/BallsAndGoals/BP_BallSpawner.BP_BallSpawner_C"))
    (`self.K2_DestroyActor` _returnvalue)
    (bind _returnvalue_2 (`|CreateWidget` "/Game/UI/W_Player2Wins.W_Player2Wins_C"))
    (`UserWidget.AddToViewport` _returnvalue_2 0)
    (`KismetSystemLibrary.Delay` 3.0)
    (goto _label)))

(event `InputAction|PauseButton` :paused true
  (params (Key :type "Key Structure"))
  (bind _returnvalue (`GameplayStatics.GetPlayerController` 0))
  (bind _pausemenu_ref (`self.PauseMenu Ref`))
  ;[1 1 1] Pause
  (:`Pressed`
    (`/Engine/EditorBlueprintResources/StandardMacros.IsValid` (`self.PauseMenu Ref`)
      (:`Is Valid`
        _)
      (:`Is Not Valid`
        (bind _returnvalue_2 (`|CreateWidget` "/Game/UI/W_PauseMenu.W_PauseMenu_C"))
        (set `self.PauseMenu Ref` _returnvalue_2)))
    (if (`GameplayStatics.IsGamePaused`)
      (`Widget.RemoveFromParent` _pausemenu_ref)
      (`GameplayStatics.SetGamePaused` false)
      (set `PlayerController.bShowMouseCursor` false _returnvalue)
      (`WidgetBlueprintLibrary.SetInputMode_GameOnly` _returnvalue)
      (else
        (`UserWidget.AddToViewport` _pausemenu_ref 0)
        (`GameplayStatics.SetGamePaused` true)
        (set `PlayerController.bShowMouseCursor` true _returnvalue)
        (`WidgetBlueprintLibrary.SetInputMode_GameAndUIEx` _returnvalue _pausemenu_ref)))))

(event `Key|M`
  (params (Key :type "Key Structure"))
  ;[1 1 1] Mute/Unmute
  (:`Pressed`
    (`/Engine/EditorBlueprintResources/StandardMacros.FlipFlop`
      (:`A`
        (`GameplayStatics.SetBaseSoundMix` "/Game/Audio/SCM_Unmute.SCM_Unmute"))
      (:`B`
        (`GameplayStatics.SetBaseSoundMix` "/Game/Audio/SCM_Mute.SCM_Mute")))))

(fn `UserConstructionScript`)