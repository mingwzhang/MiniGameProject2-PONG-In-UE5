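; NPC paddle that tracks the ball along X.
; On BeginPlay it flags its existence on BP_NPCExistCheck.
; Each Tick it loops over all BP_Ball actors, storing the sphere's relative location and calling Move, or calling Stop when BallGone is set.
; Both events drive one MoveComponentTo that eases the Cube to the ball's X over a short time, using the Cube's world Y and Z.
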(event `self.ReceiveBeginPlay`
  (bind _returnvalue (`GameplayStatics.GetActorOfClass` "/Game/Blueprint/Paddles/BP_NPCExistCheck.BP_NPCExistCheck_C"))
  (set `/Game/Blueprint/Paddles/BP_NPCExistCheck.NPC_Exist` true _returnvalue))

(event `self.ReceiveTick`
  (params (DeltaSeconds :type "Float (single-precision)"))
  ;[1 1 1] Set Up Ball Location To Follow
  (bind _outactors (`GameplayStatics.GetAllActorsOfClass` "/Game/Blueprint/BallsAndGoals/BP_Ball.BP_Ball_C"))
  (for _array_element _outactors
    (if (`self.BallGone`)
      (`self.Stop`)
      (else
        (set `self.Ball Location` (`SceneComponent.RelativeLocation` (`/Game/Blueprint/BallsAndGoals/BP_Ball.Sphere` _array_element)))
        (`self.Move`)))))

(event `Stop`
  (bind _ball_location_x (`KismetMathLibrary.BreakVector` (`self.Ball Location`)))
  (bind (_returnvalue_x _returnvalue_y _returnvalue_z) (`KismetMathLibrary.BreakVector` (`SceneComponent.K2_GetComponentLocation` (`self.Cube`))))
  ;[1 1 1] NPC Movement
  (goto _label :!via `Stop`))

(event `Move`
  (bind _ball_location_x (`KismetMathLibrary.BreakVector` (`self.Ball Location`)))
  (bind (_returnvalue_x _returnvalue_y _returnvalue_z) (`KismetMathLibrary.BreakVector` (`SceneComponent.K2_GetComponentLocation` (`self.Cube`))))
  ;[1 1 1] NPC Movement
  (`KismetSystemLibrary.MoveComponentTo` (`self.Cube`) (`KismetMathLibrary.MakeVector` _ball_location_x _returnvalue_y _returnvalue_z) (struct) false false 0.1 :!label _label))

(fn `UserConstructionScript`)