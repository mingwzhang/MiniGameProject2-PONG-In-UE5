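; BP_BallSpawner is an actor that spawns a BP_Ball at its own transform, two seconds after BeginPlay or whenever SpawnBall is called.
; After spawning, it looks up BP_NPCExistCheck and, if an NPC exists, clears the BallGone flag on the BP_NPC.
; Both actors are found with GetActorOfClass rather than stored references.
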(event `self.ReceiveBeginPlay`
  (`self.SpawnBall`))

(event `SpawnBall`
  (`KismetSystemLibrary.Delay` 2.0)
  (`|SpawnActorFromClass` "/Game/Blueprint/BallsAndGoals/BP_Ball.BP_Ball_C" (`SceneComponent.K2_GetComponentToWorld` (`self.DefaultSceneRoot`)) "Undefined" "OverrideRootScale" null null)
  (bind _returnvalue (`GameplayStatics.GetActorOfClass` "/Game/Blueprint/Paddles/BP_NPCExistCheck.BP_NPCExistCheck_C"))
  (if (`/Game/Blueprint/Paddles/BP_NPCExistCheck.NPC_Exist` _returnvalue)
    (bind _returnvalue_2 (`GameplayStatics.GetActorOfClass` "/Game/Blueprint/Paddles/BP_NPC.BP_NPC_C"))
    (set `/Game/Blueprint/Paddles/BP_NPC.BallGone` false _returnvalue_2)))

(fn `UserConstructionScript`)