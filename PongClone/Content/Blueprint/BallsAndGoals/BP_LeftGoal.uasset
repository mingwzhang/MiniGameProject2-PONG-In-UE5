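; BP_LeftGoal is the left-side goal that scores a point for the right player when a BP_Ball enters it.
; On overlap it destroys the ball, calls AddRightScore on BP_Players_Parent and flags BP_NPC if one exists.
; While the right score is below the winning score, it respawns a ball, marks a left start and plays a reset sound.
; It finds all collaborating actors through GetActorOfClass lookups.
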(event `self.ReceiveBeginPlay`)

(event `Start Left`
  (set `self.isLeftStart` true)
  (bind _returnvalue (`GameplayStatics.GetActorOfClass` "/Game/Blueprint/BallsAndGoals/BP_RightGoal.BP_RightGoal_C"))
  (set `/Game/Blueprint/BallsAndGoals/BP_RightGoal.isRightStart` false _returnvalue))

(event `self.LeftGoalCollision.OnComponentBeginOverlap`
  (params (OverlappedComponent :type "PrimitiveComponent Object Reference") (OtherActor :type "Actor Object Reference") (OtherComp :type "PrimitiveComponent Object Reference") (OtherBodyIndex :type Integer) (bFromSweep :type Boolean) (SweepResult :type "HitResult Structure (by ref)"))
  (bind _asbp_ball (cast `/Game/Blueprint/BallsAndGoals/BP_Ball` OtherActor))
  (`self.K2_DestroyActor` _asbp_ball)
  (`self.Right Gets Score`)
  (bind _returnvalue (`GameplayStatics.GetActorOfClass` "/Game/Blueprint/Paddles/BP_NPCExistCheck.BP_NPCExistCheck_C"))
  (if (`/Game/Blueprint/Paddles/BP_NPCExistCheck.NPC_Exist` _returnvalue)
    (bind _returnvalue_2 (`GameplayStatics.GetActorOfClass` "/Game/Blueprint/Paddles/BP_NPC.BP_NPC_C"))
    (set `/Game/Blueprint/Paddles/BP_NPC.BallGone` true _returnvalue_2)))

(event `Right Gets Score`
  (bind _returnvalue (`GameplayStatics.GetActorOfClass` "/Game/Blueprint/Paddles/BP_Players_Parent.BP_Players_Parent_C"))
  (`/Game/Blueprint/Paddles/BP_Players_Parent.AddRightScore` _returnvalue)
  (`self.Finish Game(Left)`))

(event `Finish Game(Left)`
  (bind _returnvalue (`GameplayStatics.GetActorOfClass` "/Game/Blueprint/Paddles/BP_Players_Parent.BP_Players_Parent_C"))
  (if (< (`/Game/Blueprint/Paddles/BP_Players_Parent.RightScore` _returnvalue) (`/Game/Blueprint/Paddles/BP_Players_Parent.ScoreToWin` _returnvalue))
    (`self.Respawn To Left`)))

(event `Respawn To Left`
  (bind _returnvalue (`GameplayStatics.GetActorOfClass` "/Game/Blueprint/BallsAndGoals/BP_BallSpawner.BP_BallSpawner_C"))
  (`/Game/Blueprint/BallsAndGoals/BP_BallSpawner.SpawnBall` _returnvalue)
  (`self.Start Left`)
  (`GameplayStatics.PlaySound2D` "/Game/Audio/resetGame.resetGame" 1.0 1.0 0.0 null null))

(fn `UserConstructionScript`)