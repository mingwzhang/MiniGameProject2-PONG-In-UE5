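; Physics-driven ball for a Pong-style game that bounces between player or NPC paddles and walls.
; On BeginPlay it reads the start flags on the left and right goals to set the Y direction of a launch impulse with random X drift.
; Sphere hits on paddles apply an opposing impulse and play a sound at world origin once per Paddle-tagged actor, while tagged walls only trigger a 2D sound.
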(event `Bounce Left`
  ;[1 1 1] Ball Hits Setting
  (`PrimitiveComponent.AddImpulse` (`self.Sphere`) (`KismetMathLibrary.MakeVector` (`KismetMathLibrary.RandomFloatInRange` -50.0 50.0) 100.0) "None" false))

(event `BounceRight`
  ;[1 1 1] Ball Hits Setting
  (`PrimitiveComponent.AddImpulse` (`self.Sphere`) (`KismetMathLibrary.MakeVector` (`KismetMathLibrary.RandomFloatInRange` -50.0 50.0) -100.0) "None" false))

(event `StartRight`
  ;[1 1 1] Initiate Ball On One of the Sides
  (bind _returnvalue (`GameplayStatics.GetActorOfClass` "/Game/Blueprint/BallsAndGoals/BP_RightGoal.BP_RightGoal_C"))
  (if (`/Game/Blueprint/BallsAndGoals/BP_RightGoal.isRightStart` _returnvalue)
    (set `self.StartingSide` 300.0)))

(event `StartLeft`
  ;[1 1 1] Initiate Ball On One of the Sides
  (bind _returnvalue (`GameplayStatics.GetActorOfClass` "/Game/Blueprint/BallsAndGoals/BP_LeftGoal.BP_LeftGoal_C"))
  (if (`/Game/Blueprint/BallsAndGoals/BP_LeftGoal.isLeftStart` _returnvalue)
    (set `self.StartingSide` -300.0)))

(event `self.Sphere.OnComponentHit`
  (params (HitComponent :type "PrimitiveComponent Object Reference") (OtherActor :type "Actor Object Reference") (OtherComp :type "PrimitiveComponent Object Reference") (NormalImpulse :type "Vector Structure") (Hit :type "HitResult Structure (by ref)"))
  ;[1 1 1] Ball Hits Setting
  (cast `/Game/Blueprint/Paddles/BP_Player1` OtherActor
    (:`then`
      (`self.Bounce Left`)
      (bind _outactors (`GameplayStatics.GetAllActorsWithTag` "Paddle" :!label _label))
      (for _ _outactors
        (`GameplayStatics.PlaySoundAtLocation` "/Game/Audio/ballHitPaddle.ballHitPaddle" (0.0 0.0 0.0) (struct) 1.0 1.0 0.0 null null null null)))
    (:`CastFailed`
      (cast `/Game/Blueprint/Paddles/BP_Player2` OtherActor
        (:`then`
          (`self.BounceRight` :!label _label_2)
          (goto _label))
        (:`CastFailed`
          (cast `/Game/Blueprint/Paddles/BP_NPC` OtherActor
            (:`then`
              (goto _label_2))
            (:`CastFailed`
              (bind _asbp_wall (cast `/Game/Blueprint/Walls/BP_Wall` OtherActor))
              (if (`self.ActorHasTag` _asbp_wall "Wall")
                (`GameplayStatics.PlaySound2D` "/Game/Audio/BallCollideWall.BallCollideWall" 1.0 1.0 0.0 null null)))))))))

(event `self.ReceiveBeginPlay`
  ;[1 1 1] Initiate Ball On One of the Sides
  (`self.StartLeft`)
  (`self.StartRight`)
  (`PrimitiveComponent.AddImpulse` (`self.Sphere`) (`KismetMathLibrary.MakeVector` (`KismetMathLibrary.RandomFloatInRange` -50.0 50.0) (`self.StartingSide`)) "None" false))

(fn `UserConstructionScript`)