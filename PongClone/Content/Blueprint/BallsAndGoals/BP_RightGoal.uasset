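; BP_RightGoal is the right-side goal, which scores a point for the left side when a ball enters it.
; Its collision overlap destroys the BP_Ball, adds to the left score on BP_Players_Parent and sets BallGone on BP_NPC if one exists.
; While the left score is below ScoreToWin, it respawns a ball, flags a right-side start and plays a reset sound.
; Other actors are found through GetActorOfClass lookups.
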(event `StartRight`
  (set `self.isRightStart` true)
  (bind _returnvalue (`GameplayStatics.GetActorOfClass` "/Game/Blueprint/BallsAndGoals/BP_LeftGoal.BP_LeftGoal_C"))
  (set `/Game/Blueprint/BallsAndGoals/BP_LeftGoal.isLeftStart` false _returnvalue))

(event `self.RightGoalCollision.OnComponentBeginOverlap`
  (params (OverlappedComponent :type "PrimitiveComponent Object Reference") (OtherActor :type "Actor Object Reference") (OtherComp :type "PrimitiveComponent Object Reference") (OtherBodyIndex :type Integer) (bFromSweep :type Boolean) (SweepResult :type "HitResult Structure (by ref)"))
  (bind _asbp_ball (cast `/Game/Blueprint/BallsAndGoals/BP_Ball` OtherActor))
  (`self.K2_DestroyActor` _asbp_ball)
  (`self.Left Gets Score`)
  (bind _returnvalue (`GameplayStatics.GetActorOfClass` "/Game/Blueprint/Paddles/BP_NPCExistCheck.BP_NPCExistCheck_C"))
  (if (`/Game/Blueprint/Paddles/BP_NPCExistCheck.NPC_Exist` _returnvalue)
    (bind _returnvalue_2 (`GameplayStatics.GetActorOfClass` "/Game/Blueprint/Paddles/BP_NPC.BP_NPC_C"))
    (set `/Game/Blueprint/Paddles/BP_NPC.BallGone` true _returnvalue_2)))

(event `Left Gets Score`
  (bind _returnvalue (`GameplayStatics.GetActorOfClass` "/Game/Blueprint/Paddles/BP_Players_Parent.BP_Players_Parent_C"))
  (`/Game/Blueprint/Paddles/BP_Players_Parent.AddLeftScore` _returnvalue)
  (`self.Finish Game (Right)`))

(event `Finish Game (Right)`
  (bind _returnvalue (`GameplayStatics.GetActorOfClass` "/Game/Blueprint/Paddles/BP_Players_Parent.BP_Players_Parent_C"))
  (if (< (`/Game/Blueprint/Paddles/BP_Players_Parent.LeftScore` _returnvalue) (`/Game/Blueprint/Paddles/BP_Players_Parent.ScoreToWin` _returnvalue))
    (`self.Spawn To Right`)))

(event `Spawn To Right`
  (bind _returnvalue (`GameplayStatics.GetActorOfClass` "/Game/Blueprint/BallsAndGoals/BP_BallSpawner.BP_BallSpawner_C"))
  (`/Game/Blueprint/BallsAndGoals/BP_BallSpawner.SpawnBall` _returnvalue)
  (`self.StartRight`)
  (`GameplayStatics.PlaySound2D` "/Game/Audio/resetGame.resetGame" 1.0 1.0 0.0 null null))

(fn `UserConstructionScript`)